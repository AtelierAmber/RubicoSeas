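; Base puppet component for units in the Advanced Turn Based Tile Toolkit, defining the queries that describe a unit's puppet.
; Its getters cover animated location, offset, name, icon, faction, move speed with acceleration, and whether the puppet is visibly dead.
; Every getter is a stub returning a fixed default or empty value, with no logic or state read in this file.
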(fn `GetAnimatedLocation`
  (returns (Location :type "Vector Structure"))
  (return (0.0 0.0 0.0)))

(fn `GetPuppetFaction`
  (returns (Faction :type "/Game/AdvancedTurnBasedTileToolkit/Core/Units/EFaction Enum"))
  (return "NewEnumerator3"))

(fn `GetPuppetIcon`
  (returns (Icon :type "Texture2D Object Reference"))
  (return null))

(fn `GetPuppetMoveSpeed`
  (returns (MoveSpeed :type "Float (double-precision)") (Acceleration :type "Float (double-precision)"))
  (return 0.0 0.0))

(fn `GetPuppetName`
  (returns (Name :type Text))
  (return ""))

(fn `GetPuppetOffset`
  (returns (Offset :type "Vector Structure"))
  (return (0.0 0.0 0.0)))

(fn `GetVisiblyDead`
  (returns (bVisiblyDead :type Boolean))
  (return false))