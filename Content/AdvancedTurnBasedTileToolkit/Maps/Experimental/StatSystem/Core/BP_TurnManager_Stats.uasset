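; Turn manager variant for the experimental stat system that broadcasts round and turn events through tag-based dispatcher hubs.
; It wraps parent logic, firing global RoundEnd before a new round and RoundStart after it.
; If another refreshed actor exists, TurnEnd fires on the active unit's hub component, or globally without a valid unit.
; TurnStart always fires globally after the parent begins the next turn, passing the active actor.
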(event `self.BeginNewRound`
  (`/Game/AdvancedTurnBasedTileToolkit/Maps/Experimental/StatSystem/Core/BPFL_DispatcherHub.CallEventInGlobalDispatcherHub` (struct :`TagName` "Event.RoundEnd") self)
  (`parent.BeginNewRound`)
  (`/Game/AdvancedTurnBasedTileToolkit/Maps/Experimental/StatSystem/Core/BPFL_DispatcherHub.CallEventInGlobalDispatcherHub` (struct :`TagName` "Event.RoundStart") self))

(event `self.ResumeAfterOngoingActionsDone`
  (`parent.ResumeAfterOngoingActionsDone`))

(event `self.BeginNextValidActorTurn`
  (params (bUseCustomDelay :type Boolean) (CustomDelay :type "Float (double-precision)"))
  (`|ExecutionSequence`
    (:`then_0`
      (bind _bfoundvalidactor (`self.FindNextRefreshedActor` false))
      (if _bfoundvalidactor
        (bind _activeunit (`self.ActiveUnit`)
          (:`then`
            (`/Game/AdvancedTurnBasedTileToolkit/Core/Events/BP_DispatcherHubComponent.CallEvent` (`self.GetComponentByClass` _activeunit "/Game/AdvancedTurnBasedTileToolkit/Core/Events/BP_DispatcherHubComponent.BP_DispatcherHubComponent_C") (struct :`TagName` "Event.TurnEnd") (`self.ActiveUnit`) null true))
          (:`else`
            (`/Game/AdvancedTurnBasedTileToolkit/Maps/Experimental/StatSystem/Core/BPFL_DispatcherHub.CallEventInGlobalDispatcherHub` (struct :`TagName` "Event.TurnEnd") self)))))
    (:`then_1`
      (`parent.BeginNextValidActorTurn` bUseCustomDelay CustomDelay)
      (`/Game/AdvancedTurnBasedTileToolkit/Maps/Experimental/StatSystem/Core/BPFL_DispatcherHub.CallEventInGlobalDispatcherHub` (struct :`TagName` "Event.TurnStart") (`self.ActiveActor`)))))

(fn `UserConstructionScript`
  (`parent.UserConstructionScript`))