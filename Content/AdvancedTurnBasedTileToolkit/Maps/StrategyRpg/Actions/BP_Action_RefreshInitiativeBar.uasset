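; BP_Action_RefreshInitiativeBar is a turn-based toolkit action for the StrategyRpg map that refreshes the on-screen initiative bar.
; When played, it casts the first player's HUD to the TRPG stats HUD and passes its Puppets to the initiative bar widget in that HUD's layout.
; It ends immediately afterward, and also ends if the HUD cast fails.
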(event `self.PlayAction`
  (bind _asbp_hud_atbtt_stats_srpg (cast `/Game/AdvancedTurnBasedTileToolkit/Maps/StrategyRpg/Core/BP_HUD_ATBTT_Stats_Trpg` (`PlayerController.GetHUD` (`GameplayStatics.GetPlayerController` 0)))
    (:`then`
      (`/Game/AdvancedTurnBasedTileToolkit/Maps/StrategyRpg/UI/WBP_InitiativeBar.RefreshInitiativeBar` (`/Game/AdvancedTurnBasedTileToolkit/Maps/StrategyRpg/UI/WBP_Layout_Trpg.WBP_InitiativeBar` (`/Game/AdvancedTurnBasedTileToolkit/Maps/StrategyRpg/Core/BP_HUD_ATBTT_Stats_Trpg.HommLayoutRef` _asbp_hud_atbtt_stats_srpg)) (`self.Puppets`))
      (`self.EndAction` true))
    (:`CastFailed`
      (`self.EndAction` true))))

(fn `UserConstructionScript`
  (`parent.UserConstructionScript`))