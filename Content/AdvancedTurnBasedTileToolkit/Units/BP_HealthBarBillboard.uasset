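; BP_HealthBarBillboard is an actor that displays a unit's health bar in the turn-based tile toolkit.
; On BeginPlay it creates a dynamic material instance from the HealthBar component's first material.
; SetHealthBarFill writes the PercentFill scalar parameter to that material and hides the actor in game when the fill is zero or below.
; GetGunMuzzle and GetPuppetCenter return only invalid or zero placeholder values.
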(event `self.ReceiveBeginPlay`
  (bind _healthbar (`self.HealthBar`))
  (bind _returnvalue (`PrimitiveComponent.CreateDynamicMaterialInstance` _healthbar 0 (`PrimitiveComponent.GetMaterial` _healthbar 0) "None"))
  (set `self.HealthBarMaterial` _returnvalue))

(event `/Game/AdvancedTurnBasedTileToolkit/Core/Units/BPI_UnitHUD.SetHealthBarFill`
  (params (PercentFill :type "Float (double-precision)"))
  (`MaterialInstanceDynamic.SetScalarParameterValue` (`self.HealthBarMaterial`) "PercentFill" PercentFill)
  (`self.SetActorHiddenInGame` (<= PercentFill 0.0)))

(fn `GetGunMuzzle`
  (returns (bValid :type Boolean) (GunComponent :type "StaticMeshComponent Object Reference") (MuzzleTransform :type "Transform Structure"))
  (return false null))

(fn `GetPuppetCenter`
  (returns (Location :type "Vector Structure"))
  (return (0.0 0.0 0.0)))

(fn `UserConstructionScript`)