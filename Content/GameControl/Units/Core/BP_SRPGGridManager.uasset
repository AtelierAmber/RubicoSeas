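; BP_SRPGGridManager is a grid manager Blueprint providing path and direction helpers for tile indexes, with no active event logic.
; ConvertGridIndexesToSplinePath turns tile indexes into offset world locations and, given a valid spline, sets them as points of a chosen type.
; ConvertIndexesToDirection looks up the index difference between two tiles in BaseEdges, returning the position as a direction enum plus a validity flag.
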(fn `ConvertGridIndexesToSplinePath`
  (params (PathIndexes :type "Array of Integer") (Offset :type "Vector Structure") (SplineIn :type "SplineComponent Object Reference") (SplineType :type "ESplinePointType Enum" :default "Linear"))
  (returns (PathLocations :type "Array of Vector Structure") (SplineOut :type "SplineComponent Object Reference"))
  (bind _locations (`self.ConvertGridIndexesToLocations` PathIndexes Offset))
  (bind _splinein (`local.SplineIn`)
    (:`then`
      (`SplineComponent.SetSplinePoints` (`local.SplineIn`) _locations "World" true)
      (for (_ _array_index) _locations
        (`SplineComponent.SetSplinePointType` (`local.SplineIn`) _array_index (`local.SplineType`) true))
      (return _locations (`local.SplineIn`)))
    (:`else`
      (return _locations _splinein))))

(fn `ConvertIndexesToDirection`
  (params (`From Tile Index` :type Integer) (`To Tile Index` :type Integer))
  (returns (`Out Direction` :type "/Game/AdvancedTurnBasedTileToolkit/Core/Grid/EDirection Enum") (Valid :type Boolean))
  (bind _returnvalue (`KismetArrayLibrary.Array_Find` (`self.BaseEdges`) (- `From Tile Index` `To Tile Index`)))
  (return (cast `/Game/AdvancedTurnBasedTileToolkit/Core/Grid/EDirection` (`KismetMathLibrary.Conv_IntToByte` _returnvalue)) (>= _returnvalue 0)))

(fn `UserConstructionScript`
  (`parent.UserConstructionScript`))