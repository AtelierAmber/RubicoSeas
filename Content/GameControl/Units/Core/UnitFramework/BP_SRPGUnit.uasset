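; Selectable SRPG grid unit that tracks which ability categories remain each turn, with one category consuming both.
; Selection notifies the turn manager and, if activation is allowed, starts the ability system or default ability; refresh restores categories and reduces cooldowns.
; Simulated tile entries queue move actions, extending the current one's path to animate continuous movement.
; GetStats and GetStatData forward to the stats component; other stat functions are stubs returning failure.
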(event `/Game/AdvancedTurnBasedTileToolkit/Core/BPI_Initiative.ExhaustActor`
  (`BlueprintSetLibrary.Set_Clear` (`self.AvailableAbilityCategories`)))

(event `/Game/AdvancedTurnBasedTileToolkit/Core/BPI_Initiative.SelectActor`
  (bind _returnvalue (`self.GetOwner` self))
  ;[0 0 0] Select Actor
  (bind ___ (`/Game/AdvancedTurnBasedTileToolkit/Core/BPML_Utility.MakeLocalVariable` (`.TurnManager` (`/Game/AdvancedTurnBasedTileToolkit/Core/BPFL_Singletons.GetTurnManager`))))
  (bind _ballowed (`/Game/AdvancedTurnBasedTileToolkit/Core/BP_TurnManager.CheckIfUnitActivationAllowed` ___ self))
  (`/Game/AdvancedTurnBasedTileToolkit/Core/BP_TurnManager.RunOnActorSelected` ___ self _ballowed)
  (`self.QueueShowUnitSelect`)
  (if _ballowed
    (if (`KismetSystemLibrary.IsValid` (`self.GetComponentByClass` self "/Game/AdvancedTurnBasedTileToolkit/Core/Units/BP_AbilitySystem.BP_AbilitySystem_C"))
      (`self.UpdateAbilityBox`)
      (`/Game/AdvancedTurnBasedTileToolkit/Core/Units/BP_AbilitySystem.ActivateUnitAbility` (`self.GetComponentByClass` self "/Game/AdvancedTurnBasedTileToolkit/Core/Units/BP_AbilitySystem.BP_AbilitySystem_C"))
      (else
        (message `/Game/AdvancedTurnBasedTileToolkit/Core/BPI_PC.ActivateAbility` (select `bool` (`KismetSystemLibrary.IsValid` _returnvalue) :`false` (`GameplayStatics.GetPlayerController` 0) :`true` _returnvalue :!type "Object Object Reference") (`self.DefaultAbility`) self true)))))

(event `/Game/AdvancedTurnBasedTileToolkit/Core/BPI_Initiative.RefreshActor`
  ;[0 0 0] Select Actor
  (`self.RefreshUnit`))

(event `self.QueueShowUnitSelect`
  (`/Game/AdvancedTurnBasedTileToolkit/Maps/Experimental/StatSystem/Core/BPFL_DispatcherHub.CallEventInGlobalDispatcherHub` (struct :`TagName` "Event.Action.UnitSelect") self)
  (`parent.QueueShowUnitSelect`))

(fn `AddToStat`
  (params (Stat :type "GameplayTag Structure") (Value :type "Float (double-precision)"))
  (returns (bSuccess :type Boolean))
  (return false))

(fn `CanPerformCombatAbility`
  (params (Ability :type "/Game/GameControl/Units/Core/Abilities/BP_AbilitySRPGCombat Object Reference"))
  (returns (Performable :type Boolean))
  (if (`|EnumEquality` (`/Game/GameControl/Units/Core/Abilities/BP_AbilitySRPGCombat.AbilityCategory` Ability) "NewEnumerator2")
    (return (and (`BlueprintSetLibrary.Set_Contains` (`self.AvailableAbilityCategories`) "NewEnumerator0") (`BlueprintSetLibrary.Set_Contains` (`self.AvailableAbilityCategories`) "NewEnumerator1")))
    (else
      (return (`BlueprintSetLibrary.Set_Contains` (`self.AvailableAbilityCategories`) "NewEnumerator0")))))

(fn `CheckIfExhausted`
  (returns (bExhausted :type Boolean))
  (return (`BlueprintSetLibrary.Set_IsEmpty` (`self.AvailableAbilityCategories`))))

(fn `GetStatData`
  (params (Stat :type "GameplayTag Structure"))
  (returns (StatData :type "/Game/AdvancedTurnBasedTileToolkit/Maps/Experimental/StatSystem/Core/FStat Structure"))
  (bind _statdata (`/Game/AdvancedTurnBasedTileToolkit/Maps/Experimental/StatSystem/Core/BP_StatsComponent.GetStatData` (`self.BP_StatsComponent`) Stat))
  (return _statdata))

(fn `GetStatMaxValue`
  (params (Stat :type "GameplayTag Structure"))
  (returns (bSuccess :type Boolean) (MaxValue :type "Float (double-precision)"))
  (return false 0.0))

(fn `GetStats`
  (returns (bSuccess :type Boolean) (Stats :type "Map of GameplayTag Structure to Float (double-precision)") (MaxStats :type "Map of GameplayTag Structure to Float (double-precision)"))
  (bind (_bsuccess _stats _maxstats) (`/Game/AdvancedTurnBasedTileToolkit/Maps/Experimental/StatSystem/Core/BP_StatsComponent.GetStats` (`self.BP_StatsComponent`)))
  (return _bsuccess _stats _maxstats))

(fn `GetStatValue`
  (params (Stat :type "GameplayTag Structure"))
  (returns (bHasStat :type Boolean) (Value :type "Float (double-precision)"))
  (return false 0.0))

(fn `MakeAbilityCategoryAvailable`
  (params (`Of Category` :type "/Game/GameControl/Units/Core/UnitFramework/ESRPGAbilityCategory Enum" :default "NewEnumerator0"))
  (`BlueprintSetLibrary.Set_Add` (`self.AvailableAbilityCategories`) `Of Category`))

(fn `MoveAlongPath`
  (params (PathIndexes :type "Array of Integer"))
  (`self.SimulateMove` PathIndexes))

(fn `PerformAbility`
  (params (`Ability Category` :type "/Game/GameControl/Units/Core/UnitFramework/ESRPGAbilityCategory Enum" :default "NewEnumerator0"))
  (bind _availableabilitycategories (`self.AvailableAbilityCategories`))
  (if (`|EnumEquality` `Ability Category` "NewEnumerator2")
    (`BlueprintSetLibrary.Set_Remove` _availableabilitycategories "NewEnumerator0")
    (`BlueprintSetLibrary.Set_Remove` _availableabilitycategories "NewEnumerator1")
    (else
      (`BlueprintSetLibrary.Set_Remove` _availableabilitycategories `Ability Category`))))

(fn `QueueOrExtendMoveAction`
  (params (ActionManager :type "/Game/AdvancedTurnBasedTileToolkit/Core/BP_ActionManager Object Reference") (MoveSource :type "Vector Structure") (MoveTarget :type "Vector Structure") (bStartOfMove :type Boolean) (bEndOfMove :type Boolean) (MoveSourceIndex :type Integer) (MoveTargetIndex :type Integer))
  (bind _localactionmanager (`self.LocalActionManager`))
  (bind _output (`|GetArrayItem` (`/Game/AdvancedTurnBasedTileToolkit/Core/BP_ActionManager.ActionQueue` _localactionmanager) (`/Game/AdvancedTurnBasedTileToolkit/Core/BP_ActionManager.FillCounter` _localactionmanager)))
  (`/Engine/EditorBlueprintResources/StandardMacros.IsValid` ActionManager
    (:`Is Valid`
      (set `self.LocalActionManager` ActionManager))
    (:`Is Not Valid`
      (set `self.LocalActionManager` (`.ActionManager` (`/Game/AdvancedTurnBasedTileToolkit/Core/BPFL_Singletons.GetActionManager`)))))
  (if (== _output (`self.CurrentMoveAction`))
    (bind _asbp_action_move (cast `/Game/AdvancedTurnBasedTileToolkit/Core/Actions/BP_Action_Move` _output)
      (:`then`
        (`KismetArrayLibrary.Array_Add` (`/Game/AdvancedTurnBasedTileToolkit/Core/Actions/BP_Action_Move.MovePath` _asbp_action_move) (`local.MoveTarget`))
        (set `/Game/AdvancedTurnBasedTileToolkit/Core/Actions/BP_Action_Move.bDecelerate` (`local.bEndOfMove`) _asbp_action_move))
      (:`CastFailed`
        (bind _returnvalue (`|SpawnActorFromClass` "/Game/GameControl/Units/Core/Actions/BP_Action_MoveDir.BP_Action_MoveDir_C" (`KismetMathLibrary.MakeTransform` (0.0 0.0 0.0)) "AlwaysSpawn" "OverrideRootScale" null (`|MakeArray` (`local.MoveSourceIndex`) (`local.MoveTargetIndex`)) (`|MakeArray` (`local.MoveSource`) (`local.MoveTarget`)) (`self.MaxSpeed`) (`self.Acceleration`) (`self.Puppet`) true (`local.bStartOfMove`) (`local.bEndOfMove`) false true -1.0 "NewEnumerator0" null :!label _label))
        (set `self.CurrentMoveAction` _returnvalue)))
    (else
      (goto _label)))
  (return))

(fn `RefreshAllStatVisuals`
  (returns (bSuccess :type Boolean))
  (return false))

(fn `RefreshUnit`
  (bind _returnvalue (`self.GetComponentByClass` self "/Game/AdvancedTurnBasedTileToolkit/Core/Units/BP_AbilitySystem.BP_AbilitySystem_C"))
  (`self.ResetPerformedAbilities`)
  (if (`KismetSystemLibrary.IsValid` _returnvalue)
    (`/Game/AdvancedTurnBasedTileToolkit/Core/Units/BP_AbilitySystem.ReduceCooldowns` _returnvalue)
    (return)
    (else
      (return))))

(fn `RemoveStatFromStatus`
  (params (Stat :type "GameplayTag Structure (by ref)") (OldValue :type "Float (double-precision) (by ref)"))
  (returns (bSuccess :type Boolean))
  (return false))

(fn `ResetPerformedAbilities`
  (set `self.AvailableAbilityCategories` (`|MakeSet` "NewEnumerator0" "NewEnumerator1" :!type "/Game/GameControl/Units/Core/UnitFramework/ESRPGAbilityCategory Enum")))

(fn `SetMaxStatToValue`
  (params (Stat :type "GameplayTag Structure") (MaxValue :type "Float (double-precision)"))
  (returns (bSuccess :type Boolean))
  (return false))

(fn `SetStatToValue`
  (params (Stat :type "GameplayTag Structure") (NewValue :type "Float (double-precision)"))
  (returns (bSuccess :type Boolean))
  (return false))

(fn `SimulateEnterTile`
  (params (EnteringGridIndex :type Integer) (ExitingGridIndex :type Integer) (PathIndexes :type "Array of Integer (by ref)"))
  (bind _gridmanagerref (`self.GridManagerRef`))
  (bind _enteringgridindex (`local.EnteringGridIndex`))
  (bind _pathindexes (`local.PathIndexes`))
  (bind _exitinggridindex (`local.ExitingGridIndex`))
  (`self.QueueOrExtendMoveAction` null (`/Game/AdvancedTurnBasedTileToolkit/Core/Grid/BP_GridManager.GetWorldLocationAtIndex` _gridmanagerref _exitinggridindex) (`/Game/AdvancedTurnBasedTileToolkit/Core/Grid/BP_GridManager.GetWorldLocationAtIndex` _gridmanagerref _enteringgridindex) (== (`|GetArrayItem` _pathindexes) (`local.ExitingGridIndex`)) (== (`|GetArrayItem` _pathindexes (`KismetArrayLibrary.Array_LastIndex` PathIndexes)) (`local.EnteringGridIndex`)) _exitinggridindex _enteringgridindex)
  (`parent.SimulateEnterTile` (`local.EnteringGridIndex`) (`local.ExitingGridIndex`) (`local.PathIndexes`))
  (return))

(fn `SubtractFromStat`
  (params (Stat :type "GameplayTag Structure") (Value :type "Float (double-precision)"))
  (returns (bSuccess :type Boolean))
  (return false))

(fn `UpdateFullStats`
  (params (Stats :type "Map of GameplayTag Structure to Float (double-precision) (by ref)") (MaxStats :type "Map of GameplayTag Structure to Float (double-precision) (by ref)"))
  (returns (bSuccess :type Boolean))
  (return false))

(fn `UpdateSpecifiedMaxStats`
  (params (MaxStats :type "Map of GameplayTag Structure to Float (double-precision)"))
  (returns (bSuccess :type Boolean))
  (return false))

(fn `UpdateSpecifiedStats`
  (params (Stats :type "Map of GameplayTag Structure to Float (double-precision)"))
  (returns (bSuccess :type Boolean))
  (return false))

(fn `UpdateStatFromStatus`
  (params (Stat :type "GameplayTag Structure (by ref)") (OldValue :type "Float (double-precision) (by ref)") (NewValue :type "Float (double-precision) (by ref)"))
  (returns (bSuccess :type Boolean))
  (return false))

(fn `UserConstructionScript`
  (`parent.UserConstructionScript`)
  (`self.ResetPerformedAbilities`))