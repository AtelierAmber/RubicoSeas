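; BP_SpriteUnit is a unit Blueprint that uses a placeholder child actor component to stand in for its puppet until the real one spawns.
; The construction script copies the placeholder's child actor class into PuppetClass, runs the parent construction, then reapplies PuppetClass to the placeholder.
; SpawnPuppet calls the parent implementation, then destroys the placeholder component.
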(event `self.SpawnPuppet`
  (`parent.SpawnPuppet`)
  (bind _placeholderpuppet (`self.PlaceholderPuppet`)
    (:`then`
      (`ActorComponent.K2_DestroyComponent` _placeholderpuppet))
    (:`else`)))

(fn `UserConstructionScript`
  (bind _output_get (set `self.PuppetClass` (`ChildActorComponent.ChildActorClass` (`self.PlaceholderPuppet`))))
  (`parent.UserConstructionScript`)
  (bind _placeholderpuppet (`self.PlaceholderPuppet`)
    (:`then`
      (`ChildActorComponent.SetChildActorClass` _placeholderpuppet _output_get))
    (:`else`)))