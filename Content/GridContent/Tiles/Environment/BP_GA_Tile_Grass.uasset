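; Grass environment tile for the grid that varies its look to hide visible tiling.
; After the parent construction script, SetupAntiTiling gives TileMesh a random quarter-turn yaw and randomly mirrors its X and Y scale.
; These rolls are unseeded, so they can change on reconstruction.
; A mesh-variant pick seeded by the anchor's grid index exists but is disconnected and never runs.
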(fn `SetupAntiTiling`
  (bind _tilemesh (`self.TileMesh`))
  (bind (_relativescale3d_x _relativescale3d_y _relativescale3d_z) (`KismetMathLibrary.BreakVector` (`SceneComponent.RelativeScale3D` _tilemesh)))
  (bind _returnvalue_x (`KismetMathLibrary.BreakVector2D` (`KismetMathLibrary.ToSign2D` (`KismetMathLibrary.MakeVector2D` (`KismetMathLibrary.Conv_IntToDouble` (`KismetMathLibrary.RandomIntegerInRange` -1))))))
  (bind _returnvalue_x_2 (`KismetMathLibrary.BreakVector2D` (`KismetMathLibrary.ToSign2D` (`KismetMathLibrary.MakeVector2D` (`KismetMathLibrary.Conv_IntToDouble` (`KismetMathLibrary.RandomIntegerInRange` -1))))))
  (`SceneComponent.K2_SetRelativeRotation` (`self.TileMesh`) (`KismetMathLibrary.MakeRotator` 0.0 0.0 (* (`KismetMathLibrary.Conv_IntToDouble` (`KismetMathLibrary.RandomIntegerInRange` 0 3)) 90.0)) false true)
  (`SceneComponent.SetRelativeScale3D` _tilemesh (`KismetMathLibrary.MakeVector` (* _relativescale3d_x _returnvalue_x) (* _relativescale3d_y _returnvalue_x_2) _relativescale3d_z)))

(fn `UserConstructionScript`
  (locals (`Random Seed` :type "RandomStream Structure"))
  (`parent.UserConstructionScript`)
  (`self.SetupAntiTiling`))