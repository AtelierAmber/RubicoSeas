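; Test grid unit that shows a placeholder child-actor puppet of its puppet class in the editor and destroys it when the real puppet spawns.
; Entering a tile during movement converts grid indices to world locations and queues puppet movement on the action manager.
; A still-current move action gets its path extended; otherwise a directional move action is spawned, accelerating only at path start and decelerating at path end.
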(event `self.SpawnPuppet`
  (`parent.SpawnPuppet`)
  (bind _placeholderpuppet (`self.PlaceholderPuppet`)
    (:`then`
      (`ActorComponent.K2_DestroyComponent` _placeholderpuppet))
    (:`else`)))

(fn `QueueOrExtendMoveAction`
  (params (ActionManager :type "/Game/AdvancedTurnBasedTileToolkit/Core/BP_ActionManager Object Reference") (MoveSource :type "Vector Structure") (MoveTarget :type "Vector Structure") (bStartOfMove :type Boolean) (bEndOfMove :type Boolean) (MoveSourceIndex :type Integer) (MoveTargetIndex :type Integer))
  (bind _localactionmanager (`self.LocalActionManager`))
  (bind _output (`|GetArrayItem` (`/Game/AdvancedTurnBasedTileToolkit/Core/BP_ActionManager.ActionQueue` _localactionmanager) (`/Game/AdvancedTurnBasedTileToolkit/Core/BP_ActionManager.FillCounter` _localactionmanager)))
  (`/Engine/EditorBlueprintResources/StandardMacros.IsValid` ActionManager
    (:`Is Valid`
      (set `self.LocalActionManager` ActionManager))
    (:`Is Not Valid`
      (set `self.LocalActionManager` (`.ActionManager` (`/Game/AdvancedTurnBasedTileToolkit/Core/BPFL_Singletons.GetActionManager`)))))
  (if (== _output (`self.CurrentMoveAction`))
    (bind _asbp_action_move (cast `/Game/AdvancedTurnBasedTileToolkit/Core/Actions/BP_Action_Move` _output)
      (:`then`
        (`KismetArrayLibrary.Array_Add` (`/Game/AdvancedTurnBasedTileToolkit/Core/Actions/BP_Action_Move.MovePath` _asbp_action_move) (`local.MoveTarget`))
        (set `/Game/AdvancedTurnBasedTileToolkit/Core/Actions/BP_Action_Move.bDecelerate` (`local.bEndOfMove`) _asbp_action_move))
      (:`CastFailed`
        (bind _returnvalue (`|SpawnActorFromClass` "/Game/GridContent/Units/Core/Actions/BP_Action_MoveDir.BP_Action_MoveDir_C" (`KismetMathLibrary.MakeTransform` (0.0 0.0 0.0)) "AlwaysSpawn" "OverrideRootScale" null (`|MakeArray` (`local.MoveSourceIndex`) (`local.MoveTargetIndex`)) (`|MakeArray` (`local.MoveSource`) (`local.MoveTarget`)) (`self.MaxSpeed`) (`self.Acceleration`) (`self.Puppet`) true (`local.bStartOfMove`) (`local.bEndOfMove`) false true -1.0 "NewEnumerator0" null :!label _label))
        (set `self.CurrentMoveAction` _returnvalue)))
    (else
      (goto _label)))
  (return))

(fn `SimulateEnterTile`
  (params (EnteringGridIndex :type Integer) (ExitingGridIndex :type Integer) (PathIndexes :type "Array of Integer (by ref)"))
  (bind _gridmanagerref (`self.GridManagerRef`))
  (bind _exitinggridindex (`local.ExitingGridIndex`))
  (bind _enteringgridindex (`local.EnteringGridIndex`))
  (bind _pathindexes (`local.PathIndexes`))
  (`self.QueueOrExtendMoveAction` null (`/Game/AdvancedTurnBasedTileToolkit/Core/Grid/BP_GridManager.GetWorldLocationAtIndex` _gridmanagerref _exitinggridindex) (`/Game/AdvancedTurnBasedTileToolkit/Core/Grid/BP_GridManager.GetWorldLocationAtIndex` _gridmanagerref _enteringgridindex) (== (`|GetArrayItem` _pathindexes) (`local.ExitingGridIndex`)) (== (`|GetArrayItem` _pathindexes (`KismetArrayLibrary.Array_LastIndex` PathIndexes)) (`local.EnteringGridIndex`)) _exitinggridindex _enteringgridindex)
  (`parent.SimulateEnterTile` (`local.EnteringGridIndex`) (`local.ExitingGridIndex`) (`local.PathIndexes`))
  (return))

(fn `UserConstructionScript`
  (`parent.UserConstructionScript`)
  (bind _placeholderpuppet (`self.PlaceholderPuppet`)
    (:`then`
      (`ChildActorComponent.SetChildActorClass` _placeholderpuppet (`self.PuppetClass`)))
    (:`else`)))