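; BP_SpriteUnit is a grid unit Blueprint that manages a placeholder for its puppet, extending a parent unit class.
; The construction script sets the PlaceholderPuppet child actor to PuppetClass, so the placeholder shows the configured puppet.
; SpawnPuppet runs the parent logic, then destroys the placeholder component if it is valid and prints the unit's GridIndex.
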(event `self.SpawnPuppet`
  (`parent.SpawnPuppet`)
  (bind _placeholderpuppet (`self.PlaceholderPuppet`)
    (:`then`
      (`ActorComponent.K2_DestroyComponent` _placeholderpuppet)
      (`KismetSystemLibrary.PrintString` (`KismetStringLibrary.Conv_IntToString` (`self.GridIndex`))))
    (:`else`)))

(fn `UserConstructionScript`
  (`parent.UserConstructionScript`)
  (bind _placeholderpuppet (`self.PlaceholderPuppet`)
    (:`then`
      (`ChildActorComponent.SetChildActorClass` _placeholderpuppet (`self.PuppetClass`)))
    (:`else`)))