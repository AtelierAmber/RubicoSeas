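; Sky actor that drives a panning-cloud sky sphere, sun light and moon light from a single sun rotation.
; The construction script creates a dynamic material and calls RefreshMaterial, which places the moon opposite the sun's pitch.
; Pitch-derived sun height samples horizon, zenith and cloud color curves, blends in stars below the horizon, and sets both light intensities.
; BeginPlay and Tick are unused, so the blueprint itself runs no day cycle.
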(fn `RefreshMaterial`
  (bind _sun_rotation (`self.Sun Rotation`))
  (bind _sky_material (`self.Sky material`))
  (bind _sun_height (`self.Sun height`))
  (bind _sun_height_2 (`self.Sun height`))
  (bind _sky_material_2 (`self.Sky material`))
  (bind _sky_material_3 (`self.Sky material`))
  (`SceneComponent.K2_SetWorldRotation` (`self.Sun Light`) (`self.Sun Rotation`) false false)
  (`SceneComponent.K2_SetWorldRotation` (`self.Moon Light`) (`KismetMathLibrary.MakeRotator` (.roll (`self.Sun Rotation`)) (+ (.pitch (`self.Sun Rotation`)) 180.0) (.yaw (`self.Sun Rotation`))) false false)
  (`|ExecutionSequence`
    (:`then_0`
      ;[1 1 1] Set Height
      (`MaterialInstanceDynamic.SetVectorParameterValue` _sky_material "Light direction" (`KismetMathLibrary.Conv_VectorToLinearColor` (`KismetMathLibrary.Conv_RotatorToVector` _sun_rotation)))
      (`MaterialInstanceDynamic.SetVectorParameterValue` _sky_material "Sun color" (`KismetMathLibrary.Conv_ColorToLinearColor` (`LightComponentBase.LightColor` (`self.Sun Light`))))
      (set `self.Sun height` (`KismetMathLibrary.MapRangeUnclamped` (.pitch _sun_rotation) 0.0 -90.0 0.0 1.0))
      (`MaterialInstanceDynamic.SetVectorParameterValue` _sky_material_2 "Horizon color" (`CurveLinearColor.GetClampedLinearColorValue` (`self.Horizon color curve`) (`self.Sun height`)))
      (`MaterialInstanceDynamic.SetVectorParameterValue` _sky_material_2 "Zenith color" (`CurveLinearColor.GetClampedLinearColorValue` (`self.Zenith color curve`) (`self.Sun height`)))
      (`MaterialInstanceDynamic.SetVectorParameterValue` _sky_material_2 "Cloud color" (`CurveLinearColor.GetClampedLinearColorValue` (`self.Cloud color curve`) _sun_height_2))
      (`MaterialInstanceDynamic.SetScalarParameterValue` _sky_material_2 "Horizon falloff" (`KismetMathLibrary.Lerp` 3.0 7.0 (`KismetMathLibrary.Abs` _sun_height_2)))
      (`MaterialInstanceDynamic.SetScalarParameterValue` _sky_material_3 "Cloud speed" (`self.Cloud speed`))
      (`MaterialInstanceDynamic.SetScalarParameterValue` _sky_material_3 "Sun brightness" (`self.Sun brightness`))
      (`MaterialInstanceDynamic.SetScalarParameterValue` _sky_material_3 "Sun height" (`KismetMathLibrary.SelectFloat` (`KismetMathLibrary.Abs` _sun_height) 0.0 (< _sun_height 0.0)))
      (`MaterialInstanceDynamic.SetScalarParameterValue` _sky_material_3 "Cloud opacity" (`self.Cloud opacity`))
      (`MaterialInstanceDynamic.SetScalarParameterValue` _sky_material_3 "Stars brightness" (`self.Stars brightness`)))
    (:`then_1`
      (`LightComponent.SetIntensity` (`self.Sun Light`) (`KismetMathLibrary.MapRangeClamped` (`self.Sun height`) 0.04 0.0 5.0))
      (`LightComponent.SetIntensity` (`self.Moon Light`) (`KismetMathLibrary.MapRangeClamped` (`self.Sun height`) 0.0 -0.04 0.0 (`self.Moon brightness`))))))

(fn `UserConstructionScript`
  (bind _returnvalue (`PrimitiveComponent.CreateDynamicMaterialInstance` (`self.Sky Sphere`) 0 "/Engine/EngineSky/M_Sky_Panning_Clouds2.M_Sky_Panning_Clouds2" "None"))
  (set `self.Sky material` _returnvalue)
  (`self.RefreshMaterial`))